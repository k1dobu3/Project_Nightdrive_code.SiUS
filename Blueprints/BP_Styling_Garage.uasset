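; Garage trigger for visual car styling: an overlapping BP_Sedan_Chaos1 is parked, teleported inside and switched to its garage camera behind a loading animation.
; Left/right inputs step the camera through preset transforms, and the current index decides which part up/down edits.
; SelectUp and SelectDown swap front bumper, back bumper or hood (Cupot) meshes from arrays.
; Backspace teleports the car out, restoring driving camera and speedometer.
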(event EventBeginPlay
  (Input|DisableInput (Game|GetPlayerController 0)))

(event Collision|EventActorBeginOverlap
  (params (OtherActor :type Actor%20Object%20Reference))
  (Input|EnableInput (Game|GetPlayerController 0))
  (bind _asbp_sedan_chaos_1 (Utilities|Casting|CastToBP_Sedan_Chaos1 OtherActor))
  (Variables|Default|SetCameraArray_Count 0)
  (bind _asrace_ui (Utilities|Casting|CastToRaceUI (HUD|GetHUD (Game|GetPlayerController 0))))
  (Class|ChaosVehicleMovementComponent|SetParked (Variables|/Script/ChaosVehicles.WheeledVehiclePawn|GetVehicleMovementComponent _asbp_sedan_chaos_1) true)
  (Default|LoadingAnimation (Variables|/Game/Blueprints/UI_BP/RaceUI.RaceUI_C|GetUI_Ref _asrace_ui))
  (Utilities|FlowControl|Delay 1.5)
  (Default|ShowPodzkazka (Variables|/Game/Blueprints/UI_BP/RaceUI.RaceUI_C|GetUI_Ref _asrace_ui))
  (Default|HideSpeedometr (Variables|/Game/Blueprints/UI_BP/RaceUI.RaceUI_C|GetUI_Ref _asrace_ui))
  (Transformation|Teleport OtherActor "4093.000000,6723.000000,-1.000000" "0.000000,-20.000000,0.000000")
  (Components|Activation|SetActive (Variables|/Game/VehicleVarietyVol2/Blueprints/Sedan/BP_Sedan_Chaos1.BP_Sedan_Chaos1_C|GetGarageCamera _asbp_sedan_chaos_1) true false)
  (Components|Activation|SetActive (Variables|/Game/VehicleVarietyVol2/Blueprints/Sedan/BP_Sedan_Chaos1.BP_Sedan_Chaos1_C|GetCamera _asbp_sedan_chaos_1) false false)
  (Transformation|SetRelativeTransform (Variables|/Game/VehicleVarietyVol2/Blueprints/Sedan/BP_Sedan_Chaos1.BP_Sedan_Chaos1_C|GetGarageCamera _asbp_sedan_chaos_1) (Math|Transform|MakeTransform "1100.000000,320.000000,0.000000" "-10.000000,-140.000000,0.000000" "1.000000,1.000000,1.000000") false false))

(event Input|ActionEvents|InputActionGarageStylingSelectUp
  (params (Key :type Key%20Structure :default "None"))
  (:Pressed
    (CallFunction|SelectUp (Variables|/Game/VehicleVarietyVol2/Blueprints/Sedan/BP_Sedan_Chaos1.BP_Sedan_Chaos1_C|GetFrontBumper (stale Collision|EventActorBeginOverlap _asbp_sedan_chaos_1)) (Variables|/Game/VehicleVarietyVol2/Blueprints/Sedan/BP_Sedan_Chaos1.BP_Sedan_Chaos1_C|GetBackBumper (stale Collision|EventActorBeginOverlap _asbp_sedan_chaos_1)) (Variables|/Game/VehicleVarietyVol2/Blueprints/Sedan/BP_Sedan_Chaos1.BP_Sedan_Chaos1_C|GetCupot (stale Collision|EventActorBeginOverlap _asbp_sedan_chaos_1)))))

(event Input|ActionEvents|InputActionGarageStylingSelectDown
  (params (Key :type Key%20Structure :default "None"))
  (:Pressed
    (CallFunction|SelectDown (Variables|/Game/VehicleVarietyVol2/Blueprints/Sedan/BP_Sedan_Chaos1.BP_Sedan_Chaos1_C|GetFrontBumper (stale Collision|EventActorBeginOverlap _asbp_sedan_chaos_1)) (Variables|/Game/VehicleVarietyVol2/Blueprints/Sedan/BP_Sedan_Chaos1.BP_Sedan_Chaos1_C|GetBackBumper (stale Collision|EventActorBeginOverlap _asbp_sedan_chaos_1)) (Variables|/Game/VehicleVarietyVol2/Blueprints/Sedan/BP_Sedan_Chaos1.BP_Sedan_Chaos1_C|GetCupot (stale Collision|EventActorBeginOverlap _asbp_sedan_chaos_1)))))

(event Input|ActionEvents|InputActionGarage_Navigatiob_Right
  (params (Key :type Key%20Structure :default "None"))
  (:Pressed
    (if (not (== (Variables|Default|GetCameraArray_Count) 5))
      (bind _output_get (Variables|Default|SetCameraArray_Count (+ (Variables|Default|GetCameraArray_Count) 1)))
      (Transformation|SetRelativeTransform (Variables|/Game/VehicleVarietyVol2/Blueprints/Sedan/BP_Sedan_Chaos1.BP_Sedan_Chaos1_C|GetGarageCamera (stale Collision|EventActorBeginOverlap _asbp_sedan_chaos_1)) (Utilities|Array|Get(acopy) (Variables|Default|GetCameraTransform_Array) _output_get) false false))))

(event Input|ActionEvents|InputActionGarage_Navigatiob_Left
  (params (Key :type Key%20Structure :default "None"))
  (:Pressed
    (if (not (== (Variables|Default|GetCameraArray_Count) 0))
      (bind _output_get (Variables|Default|SetCameraArray_Count (- (Variables|Default|GetCameraArray_Count) 1)))
      (Transformation|SetRelativeTransform (Variables|/Game/VehicleVarietyVol2/Blueprints/Sedan/BP_Sedan_Chaos1.BP_Sedan_Chaos1_C|GetGarageCamera (stale Collision|EventActorBeginOverlap _asbp_sedan_chaos_1)) (Utilities|Array|Get(acopy) (Variables|Default|GetCameraTransform_Array) _output_get) false false))))

(event Input|KeyboardEvents|Backspace
  (params (Key :type Key%20Structure :default "None"))
  (:Pressed
    (Default|LoadingAnimation (Variables|/Game/Blueprints/UI_BP/RaceUI.RaceUI_C|GetUI_Ref (stale Collision|EventActorBeginOverlap _asrace_ui)))
    (Utilities|FlowControl|Delay 1.5)
    (Class|ChaosVehicleMovementComponent|SetParked (Variables|/Script/ChaosVehicles.WheeledVehiclePawn|GetVehicleMovementComponent (stale Collision|EventActorBeginOverlap _asbp_sedan_chaos_1)) false)
    (Transformation|Teleport (stale Collision|EventActorBeginOverlap OtherActor) "5561.000000,6690.000000,-1.000000" "0, 0, 0")
    (Components|Activation|SetActive (Variables|/Game/VehicleVarietyVol2/Blueprints/Sedan/BP_Sedan_Chaos1.BP_Sedan_Chaos1_C|GetGarageCamera (stale Collision|EventActorBeginOverlap _asbp_sedan_chaos_1)) false false)
    (Components|Activation|SetActive (Variables|/Game/VehicleVarietyVol2/Blueprints/Sedan/BP_Sedan_Chaos1.BP_Sedan_Chaos1_C|GetCamera (stale Collision|EventActorBeginOverlap _asbp_sedan_chaos_1)) true false)
    (Default|HidPodzkazka (Variables|/Game/Blueprints/UI_BP/RaceUI.RaceUI_C|GetUI_Ref (stale Collision|EventActorBeginOverlap _asrace_ui)))
    (Default|ShowSpeedometr (Variables|/Game/Blueprints/UI_BP/RaceUI.RaceUI_C|GetUI_Ref (stale Collision|EventActorBeginOverlap _asrace_ui)))))

(fn ConstructionScript)

(fn SelectUp
  (params (FrontBumper :type Static%20Mesh%20Component%20Object%20Reference) (BackBumper :type Static%20Mesh%20Component%20Object%20Reference) (Cupot :type Static%20Mesh%20Component%20Object%20Reference) (Disk :type Static%20Mesh%20Component%20Object%20Reference))
  (bind _cameraarray_count (Variables|Default|GetCameraArray_Count))
  (Utilities|FlowControl|Sequence
    (:then_0
      (if (== _cameraarray_count 1)
        (if (not (== (Variables|Default|GetFrontBumperIndex) 1))
          (bind _output_get (Variables|Default|SetFrontBumperIndex (+ (Variables|Default|GetFrontBumperIndex) 1)))
          (Components|StaticMesh|SetStaticMesh FrontBumper (Utilities|Array|Get(acopy) (Variables|Default|GetFrontBumperArray) _output_get)))))
    (:then_1
      (if (== _cameraarray_count 2)
        (if (not (== (Variables|Default|GetBackBumperIndex) 1))
          (bind _output_get_2 (Variables|Default|SetBackBumperIndex (+ (Variables|Default|GetBackBumperIndex) 1)))
          (Components|StaticMesh|SetStaticMesh BackBumper (Utilities|Array|Get(acopy) (Variables|Default|GetBackBumperArray) _output_get_2)))))
    (:then_2
      (if (== _cameraarray_count 4)
        (if (not (== (Variables|Default|GetCupotIndex) 1))
          (bind _output_get_3 (Variables|Default|SetCupotIndex (+ (Variables|Default|GetCupotIndex) 1)))
          (Components|StaticMesh|SetStaticMesh Cupot (Utilities|Array|Get(acopy) (Variables|Default|GetCupotArray) _output_get_3)))))))

(fn SelectDown
  (params (FrontBumper :type Static%20Mesh%20Component%20Object%20Reference) (Backbumper :type Static%20Mesh%20Component%20Object%20Reference) (Cupot :type Static%20Mesh%20Component%20Object%20Reference) (Disk :type Static%20Mesh%20Component%20Object%20Reference))
  (bind _cameraarray_count (Variables|Default|GetCameraArray_Count))
  (Utilities|FlowControl|Sequence
    (:then_0
      (if (== _cameraarray_count 1)
        (if (not (== (Variables|Default|GetFrontBumperIndex) 0))
          (bind _output_get (Variables|Default|SetFrontBumperIndex (- (Variables|Default|GetFrontBumperIndex) 1)))
          (Components|StaticMesh|SetStaticMesh FrontBumper (Utilities|Array|Get(acopy) (Variables|Default|GetFrontBumperArray) _output_get)))))
    (:then_1
      (if (== _cameraarray_count 2)
        (if (not (== (Variables|Default|GetBackBumperIndex) 0))
          (bind _output_get_2 (Variables|Default|SetBackBumperIndex (- (Variables|Default|GetBackBumperIndex) 1)))
          (Components|StaticMesh|SetStaticMesh Backbumper (Utilities|Array|Get(acopy) (Variables|Default|GetBackBumperArray) _output_get_2)))))
    (:then_2
      (if (== _cameraarray_count 4)
        (if (not (== (Variables|Default|GetCupotIndex) 0))
          (bind _output_get_3 (Variables|Default|SetCupotIndex (- (Variables|Default|GetCupotIndex) 1)))
          (Components|StaticMesh|SetStaticMesh Cupot (Utilities|Array|Get(acopy) (Variables|Default|GetCupotArray) _output_get_3)))))))