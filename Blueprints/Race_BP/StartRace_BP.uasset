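; StartRace_BP is a race start trigger that moves the player's car into a streamed race level when overlapped.
; On overlap it plays the RaceUI loading animation, parks the Chaos sedan, and after a short delay disables pawn input.
; It then starts a non-blocking load of the level named by RaceName, immediately teleports the controlled pawn to a configured transform and shows the HUD.
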(event Collision|EventActorBeginOverlap
  (params (OtherActor :type Actor%20Object%20Reference))
  (bind _asrace_ui (Utilities|Casting|CastToRaceUI (HUD|GetHUD (Game|GetPlayerController 0))))
  (Default|LoadingAnimation (Variables|/Game/Blueprints/UI_BP/RaceUI.RaceUI_C|GetUI_Ref _asrace_ui))
  (bind _asbp_sedan_chaos_1 (Utilities|Casting|CastToBP_Sedan_Chaos1 OtherActor))
  (Class|ChaosVehicleMovementComponent|SetParked (Variables|/Script/ChaosVehicles.WheeledVehiclePawn|GetVehicleMovementComponent _asbp_sedan_chaos_1) true)
  (Utilities|FlowControl|Delay 1.5)
  (Input|DisableInput (Game|Player|GetPlayerPawn 0) (Game|GetPlayerController 0))
  (Game|LoadStreamLevel(byName) (Variables|Default|GetRace_Name) true)
  (Transformation|Teleport (Pawn|GetControlledPawn (Game|GetPlayerController 0)) (Variables|Default|GetTP_Vector) (Variables|Default|GetTP_Roatation))
  (Default|ShowHUD (Variables|/Game/Blueprints/UI_BP/RaceUI.RaceUI_C|GetUI_Ref _asrace_ui)))

(fn ConstructionScript)