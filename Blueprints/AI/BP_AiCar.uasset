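; BP_AiCar is an AI car that exposes driving controls and state for external logic, with no decision-making in its own graphs.
; Events pass throttle, steering and brake inputs straight to the vehicle movement component, while a separate event toggles two point lights as brake lights.
; Getters return the front, left and right collision boxes, plus forward speed converted from cm/s to km/h.
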(event EventSetBreakLight
  (params (BreakeLight :type Boolean))
  (Rendering|SetVisibility (Variables|Default|GetPointLight1) BreakeLight false))

(event EventSetThrottle
  (params (Tgrottle :type Float%20%28double-precision%29))
  (Class|ChaosVehicleMovementComponent|SetThrottleInput (Variables|Default|GetVehicleMovementComponent) Tgrottle))

(event EventSetSteering
  (params (Steering :type Float%20%28double-precision%29))
  (Class|ChaosVehicleMovementComponent|SetSteeringInput (Variables|Default|GetVehicleMovementComponent) Steering))

(event EventSetBrake
  (params (Breake :type Float%20%28double-precision%29))
  (Class|ChaosVehicleMovementComponent|SetBrakeInput (Variables|Default|GetVehicleMovementComponent) Breake))

(fn ConstructionScript)

(fn GetCollisionBoxes
  (return (Variables|Default|GetFrontBox) (Variables|Default|GetLeftSideBox) (Variables|Default|GetRightSideBox)))

(fn GetCurrectSpeed
  (return (* (Vehicle|GetForwardSpeed (Variables|Default|GetVehicleMovementComponent)) 0.036)))